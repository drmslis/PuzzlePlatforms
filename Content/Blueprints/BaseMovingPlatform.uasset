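; Base moving platform Blueprint that shows whether it is active through its PointLight; the graph itself contains no movement logic.
; Each Tick checks IsActive, turning the light green when active and red when inactive.
; Two DoOnce gates reset each other so the color is set only on a state change.
; While active, the PointLight also rolls at MechRotationSpeed, scaled by delta time.
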(event `self.ReceiveTick`
  (params (DeltaSeconds :type "Float (single-precision)"))
  (if (`self.IsActive`)
    (`|ExecutionSequence`
      (:`then_0`
        (`/Engine/EditorBlueprintResources/StandardMacros.DoOnce` false :!label _label
          (:`Completed`
            (`LightComponent.SetLightColor` (`self.PointLight`) (struct :`R` 0.056746 :`G` 0.546875 :`B` 0.003751 :`A` 1.0) true)
            (goto _label_2 :!via `Reset`))))
      (:`then_1`
        (`SceneComponent.K2_AddLocalRotation` (`self.PointLight`) (`KismetMathLibrary.MakeRotator` (* DeltaSeconds (`self.MechRotationSpeed`))) false false)))
    (else
      (`/Engine/EditorBlueprintResources/StandardMacros.DoOnce` false :!label _label_2
        (:`Completed`
          (`LightComponent.SetLightColor` (`self.PointLight`) (struct :`R` 0.546875 :`G` 0.004791 :`A` 1.0) true)
          (goto _label :!via `Reset`))))))

(fn `UserConstructionScript`)